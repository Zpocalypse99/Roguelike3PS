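; Base melee weapon Blueprint that damages actors overlapping its HitBox during a timed attack window.
; PrimaryAttack clears the hit list, enables query-only collision and starts timers to close the window and call ResetAttack after a cooldown.
; Overlaps skip the owner and damage each actor once per swing, printing a debug message.
; ResetAttack sets CanAttack to false, so nothing here re-arms the attack.
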(event `self.HitBox.OnComponentBeginOverlap`
  (params (OverlappedComponent :type "PrimitiveComponent Object Reference") (OtherActor :type "Actor Object Reference") (OtherComp :type "PrimitiveComponent Object Reference") (OtherBodyIndex :type Integer) (bFromSweep :type Boolean) (SweepResult :type "HitResult Structure (by ref)"))
  (if (== (`self.OwnerCharacter`) OtherActor)
    _
    (elif (not (`KismetArrayLibrary.Array_Contains` (`self.AlreadyHitActors`) OtherActor))
      (`KismetArrayLibrary.Array_AddUnique` (`self.AlreadyHitActors`) OtherActor)
      (`GameplayStatics.ApplyDamage` OtherActor (`self.MaleeDamage`) null self)
      (`KismetSystemLibrary.PrintString` "hit"))))

(fn `EndAttackWindow`
  (`PrimitiveComponent.SetCollisionEnabled` (`self.HitBox`) "NoCollision"))

(fn `PrimaryAttack`
  (if (`self.CanAttack`)
    (set `self.CanAttack` false)
    (`KismetArrayLibrary.Array_Clear` (`self.AlreadyHitActors`))
    (`PrimitiveComponent.SetCollisionEnabled` (`self.HitBox`) "QueryOnly")
    (`KismetSystemLibrary.K2_SetTimer` self "EndAttackWindow" (`self.AttackWindow`))
    (`KismetSystemLibrary.K2_SetTimer` null "ResetAttack" (+ (`self.AttackWindow`) (`self.AttackCooldown`)))))

(fn `ResetAttack`
  (set `self.CanAttack` false))

(fn `UserConstructionScript`
  (`parent.UserConstructionScript`))