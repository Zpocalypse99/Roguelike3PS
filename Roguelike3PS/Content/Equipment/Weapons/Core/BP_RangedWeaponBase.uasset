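; Base Blueprint for ranged weapons, providing hitscan firing with an ammo count and timed reloading.
; PrimaryAttack, blocked while reloading or empty, spends a round, line traces forward from MuzzlePoint on Visibility and applies damage to the hit actor.
; Reload checks CanReload, holds the IsReloading flag through a delay, then refills the ammo.
; Debug trace drawing and hit, miss and reload prints are left in for feedback.
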(event `Reload`
  (bind _canreload (`self.CanReload`))
  (if _canreload
    (set `self.bIsReloading` true)
    (`KismetSystemLibrary.Delay` (`self.ReloadTime`))
    (`self.FinishReload`)))

(event `FinishReload`
  (set `self.CurrentAmmo` (`self.MaxAmmo`))
  (set `self.bIsReloading` false)
  (`KismetSystemLibrary.PrintString` "Reloaded"))

(fn `CanReload`
  (returns (CanReload :type Boolean))
  (return (and (not (`self.bIsReloading`)) (< (`self.CurrentAmmo`) (`self.MaxAmmo`)))))

(fn `PrimaryAttack`
  (bind _returnvalue (`SceneComponent.K2_GetComponentLocation` (`self.MuzzlePoint`)))
  (if (`self.bIsReloading`)
    _
    (elif (> (`self.CurrentAmmo`) 0)
      (set `self.CurrentAmmo` (- (`self.CurrentAmmo`) 1))
      (bind (_outhit _returnvalue_2) (`KismetSystemLibrary.LineTraceSingle` :`Start` _returnvalue :`End` (+ _returnvalue (* (`SceneComponent.GetForwardVector` (`self.MuzzlePoint`)) (`self.FireRange`))) :`TraceChannel` "TraceTypeQuery1" :`DrawDebugType` "ForDuration"))
      (if _returnvalue_2
        (`GameplayStatics.ApplyDamage` (`.HitActor` (`GameplayStatics.BreakHitResult` _outhit)) (`self.BaseDamage`) null self)
        (`KismetSystemLibrary.PrintString` "Hit")
        (else
          (`KismetSystemLibrary.PrintString` "Miss"))))))

(fn `UserConstructionScript`
  (`parent.UserConstructionScript`))