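; Weapon pedestal actor that displays a weapon and lets the player equip it.
; On BeginPlay it spawns an actor of WeaponClass and attaches it to WeaponPoint.
; Overlapping InteractionBox registers the pedestal as the BP_BasePlayer's CurrentInteractablePedestal, clearing it on exit only if still current.
; SelectWeapon passes WeaponClass to EquipWeapon on player 0's character, leaving the displayed actor in place.
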(event `self.ReceiveBeginPlay`
  (bind _returnvalue (`|SpawnActorFromClass` (`self.WeaponClass`) (`SceneComponent.K2_GetComponentToWorld` (`self.WeaponPoint`)) "Undefined" "MultiplyWithRoot" null null))
  (`self.K2_AttachToComponent` _returnvalue (`self.WeaponPoint`) "None" "SnapToTarget" "SnapToTarget" "KeepRelative" false))

(event `self.InteractionBox.OnComponentBeginOverlap`
  (params (OverlappedComponent :type "PrimitiveComponent Object Reference") (OtherActor :type "Actor Object Reference") (OtherComp :type "PrimitiveComponent Object Reference") (OtherBodyIndex :type Integer) (bFromSweep :type Boolean) (SweepResult :type "HitResult Structure (by ref)"))
  (bind _asbp_base_player (cast `/Game/Actors/BP_BasePlayer` OtherActor))
  (set `/Game/Actors/BP_BasePlayer.CurrentInteractablePedestal` self _asbp_base_player))

(event `self.InteractionBox.OnComponentEndOverlap`
  (params (OverlappedComponent :type "PrimitiveComponent Object Reference") (OtherActor :type "Actor Object Reference") (OtherComp :type "PrimitiveComponent Object Reference") (OtherBodyIndex :type Integer))
  (bind _asbp_base_player (cast `/Game/Actors/BP_BasePlayer` OtherActor))
  (if (== (`/Game/Actors/BP_BasePlayer.CurrentInteractablePedestal` _asbp_base_player) self)
    (set `/Game/Actors/BP_BasePlayer.CurrentInteractablePedestal` null _asbp_base_player)))

(event `SelectWeapon`
  (bind _asbp_base_player (cast `/Game/Actors/BP_BasePlayer` (`GameplayStatics.GetPlayerCharacter` 0)))
  (`/Game/Actors/BP_BasePlayer.EquipWeapon` _asbp_base_player (`self.WeaponClass`)))

(fn `UserConstructionScript`)