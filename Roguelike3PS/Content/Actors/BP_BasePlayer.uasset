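; Base player character that handles Enhanced Input movement, look, jump and firing the current weapon's primary attack.
; BeginPlay caches the controller and animation Blueprint, binds the health component's hurt event, and spawns the starting weapon on the right-hand socket.
; Death handling disables collision and input, while hurt handling is an empty stub.
; Debug keys add EXP and print StatSystem primary and secondary stats.
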(event Input|EnhancedActionEvents|EnhancedInputActionIA_Look
  (params (ActionValue :type Vector%202D%20Structure) (ElapsedSeconds :type Float%20%28double-precision%29) (TriggeredSeconds :type Float%20%28double-precision%29) (InputAction :type Input%20Action%20Object%20Reference :default "/Game/Input/IA_Look.IA_Look"))
  ;[0.008024 1 0.8514 0.5] Input
  (Pawn|Input|AddControllerYawInput (.x ActionValue))
  (Pawn|Input|AddControllerPitchInput (.y ActionValue)))

(event Input|EnhancedActionEvents|EnhancedInputActionIA_MoveForward
  (params (ActionValue :type Float%20%28double-precision%29) (ElapsedSeconds :type Float%20%28double-precision%29) (TriggeredSeconds :type Float%20%28double-precision%29) (InputAction :type Input%20Action%20Object%20Reference :default "/Game/Input/IA_MoveForward.IA_MoveForward"))
  ;[0.008024 1 0.8514 0.5] Input
  (Pawn|Input|AddMovementInput (Math|Vector|GetForwardVector (Math|Rotator|MakeRotator 0.0 0.0 (.yaw (Pawn|GetControlRotation :!class /Script/Engine.Pawn)))) ActionValue false))

(event Input|EnhancedActionEvents|EnhancedInputActionIA_MoveRight
  (params (ActionValue :type Float%20%28double-precision%29) (ElapsedSeconds :type Float%20%28double-precision%29) (TriggeredSeconds :type Float%20%28double-precision%29) (InputAction :type Input%20Action%20Object%20Reference :default "/Game/Input/IA_MoveRight.IA_MoveRight"))
  ;[0.008024 1 0.8514 0.5] Input
  (Pawn|Input|AddMovementInput (Math|Vector|GetRightVector (Math|Rotator|MakeRotator 0.0 0.0 (.yaw (Pawn|GetControlRotation :!class /Script/Engine.Pawn)))) ActionValue false))

(event Input|EnhancedActionEvents|EnhancedInputActionIA_Jump
  (params (ActionValue :type Boolean) (ElapsedSeconds :type Float%20%28double-precision%29) (TriggeredSeconds :type Float%20%28double-precision%29) (InputAction :type Input%20Action%20Object%20Reference :default "/Game/Input/IA_Jump.IA_Jump"))
  ;[0.008024 1 0.8514 0.5] Input
  (:Started
    (Character|Jump))
  (:Canceled
    (Character|StopJumping :!label _label))
  (:Completed
    (goto _label)))

(event Input|EnhancedActionEvents|EnhancedInputActionIA_Fire
  (params (ActionValue :type Boolean) (ElapsedSeconds :type Float%20%28double-precision%29) (TriggeredSeconds :type Float%20%28double-precision%29) (InputAction :type Input%20Action%20Object%20Reference :default "/Game/Input/IA_Fire.IA_Fire"))
  (bind _currentweapon (Variables|Default|GetCurrentWeapon))
  ;[0.008024 1 0.8514 0.5] Input
  (:Started
    (Utilities|IsValid _currentweapon
      (:Is%20Valid
        (Default|PrimaryAttack _currentweapon)))))

(event EventBeginPlay
  (|CallParentFunction)
  (bind _asplayer_controller (Utilities|Casting|CastToPlayerController (Pawn|GetController))
    (:then
      (Variables|Default|SetPlayer%20Controller _asplayer_controller)
      (bind _asabp_player_animation (Utilities|Casting|CastToABP_PlayerAnimation (Components|SkeletalMesh|GetAnimInstance (Variables|Character|GetMesh)))
        (:then
          (Variables|Default|SetAnimBP _asabp_player_animation)
          (EventDispatchers|BindEventtoOnHurt (Variables|Default|GetHealthComponent) (EventDispatchers|CreateEvent :!event HandleHurt))
          (bind _returnvalue (Game|SpawnActorfromClass (Variables|Default|GetStartingWeaponClass) (Math|Transform|MakeTransform "0, 0, 0") "Undefined" "MultiplyWithRoot" 0 0))
          (Variables|Default|SetCurrentWeapon _returnvalue)
          (Transformation|AttachComponentToComponent (Variables|Default|GetCurrentWeapon) (Variables|Character|GetMesh) "hand_r_socket" "SnapToTarget" "SnapToTarget" "KeepRelative" false))
        (:CastFailed
          (Development|PrintString "Failed to find Player Anim Instance"))))
    (:CastFailed
      (Development|PrintString "Failed to find Player Controller")
      (Actor|DestroyActor))))

(event Input|KeyboardEvents|DebugKey1
  (params (Key :type Key%20Structure :default "None") (ActionValue :type Input%20Action%20Value%20Structure))
  ;[0.15 0 0.003723 0.5] DEBUG FUNCTIONS to test if EXP and stats are working correctly
  (:Pressed
    (Development|PrintString (Utilities|String|Append "Level: " (Utilities|String|ToString(Float) (.StatValue (Default|CheckPrimaryStats (Variables|Default|GetStatSystem) "NewEnumerator3")))) true true "(R=0.000000,G=0.660000,B=1.000000,A=1.000000)" 1e+01)
    (Development|PrintString (Utilities|String|Append "MaxHealth: " (Utilities|String|ToString(Float) (.StatValue (Default|CheckPrimaryStats (Variables|Default|GetStatSystem) "NewEnumerator10")))) true true "(R=0.000000,G=0.660000,B=1.000000,A=1.000000)" 1e+01)
    (Development|PrintString (Utilities|String|Append "Strength: " (Utilities|String|ToString(Float) (.StatValue (Default|CheckPrimaryStats (Variables|Default|GetStatSystem) "NewEnumerator1")))) true true "(R=0.000000,G=0.660000,B=1.000000,A=1.000000)" 1e+01)
    (Development|PrintString (Utilities|String|Append "Defence: " (Utilities|String|ToString(Float) (.StatValue (Default|CheckPrimaryStats (Variables|Default|GetStatSystem) "NewEnumerator2")))) true true "(R=0.000000,G=0.660000,B=1.000000,A=1.000000)" 1e+01)
    (Development|PrintString (Utilities|String|Append "Magic: " (Utilities|String|ToString(Float) (.StatValue (Default|CheckPrimaryStats (Variables|Default|GetStatSystem) "NewEnumerator6")))) true true "(R=0.000000,G=0.660000,B=1.000000,A=1.000000)" 1e+01)
    (Development|PrintString (Utilities|String|Append "Resistance: " (Utilities|String|ToString(Float) (.StatValue (Default|CheckPrimaryStats (Variables|Default|GetStatSystem) "NewEnumerator7")))) true true "(R=0.000000,G=0.660000,B=1.000000,A=1.000000)" 1e+01)
    (Development|PrintString (Utilities|String|Append "Speed: " (Utilities|String|ToString(Float) (.StatValue (Default|CheckPrimaryStats (Variables|Default|GetStatSystem) "NewEnumerator8")))) true true "(R=0.000000,G=0.660000,B=1.000000,A=1.000000)" 1e+01)))

(event Input|KeyboardEvents|DebugKey2
  (params (Key :type Key%20Structure :default "None") (ActionValue :type Input%20Action%20Value%20Structure))
  ;[0.15 0 0.003723 0.5] DEBUG FUNCTIONS to test if EXP and stats are working correctly
  (:Pressed
    (Development|PrintString (Utilities|String|Append "Level: " (Utilities|String|ToString(Float) (.StatValue (Default|CheckPrimaryStats (Variables|Default|GetStatSystem) "NewEnumerator3")))) true true "(R=0.000000,G=0.660000,B=1.000000,A=1.000000)" 1e+01)
    (Development|PrintString (Utilities|String|Append "Attack Speed:" (Utilities|String|ToString(Float) (.StatValue (Default|CheckSecondaryStats (Variables|Default|GetStatSystem) "NewEnumerator6")))) true true "(R=0.000000,G=0.660000,B=1.000000,A=1.000000)" 1e+01)
    (Development|PrintString (Utilities|String|Append "Physical Damage:" (Utilities|String|ToString(Float) (.StatValue (Default|CheckSecondaryStats (Variables|Default|GetStatSystem) "NewEnumerator7")))) true true "(R=0.000000,G=0.660000,B=1.000000,A=1.000000)" 1e+01)
    (Development|PrintString (Utilities|String|Append "Magic Damage: " (Utilities|String|ToString(Float) (.StatValue (Default|CheckSecondaryStats (Variables|Default|GetStatSystem) "NewEnumerator8")))) true true "(R=0.000000,G=0.660000,B=1.000000,A=1.000000)" 1e+01)
    (Development|PrintString (Utilities|String|Append "Status Resistance: " (Utilities|String|ToString(Float) (.StatValue (Default|CheckSecondaryStats (Variables|Default|GetStatSystem) "NewEnumerator9")))) true true "(R=0.000000,G=0.660000,B=1.000000,A=1.000000)" 1e+01)))

(event Input|KeyboardEvents|Q
  (params (Key :type Key%20Structure :default "None"))
  ;[0.15 0 0.003723 0.5] DEBUG FUNCTIONS to test if EXP and stats are working correctly
  (:Pressed
    (bind _value (Default|AddPrimaryStatValue (Variables|Default|GetStatSystem) "NewEnumerator4" 5e+01))
    (Development|PrintString (Utilities|String|Append "Current EXP: " (Utilities|String|ToString(Float) _value)))
    (Development|PrintString (Utilities|String|Append "Current Level: " (Utilities|String|ToString(Float) (.StatValue (Default|CheckPrimaryStats (Variables|Default|GetStatSystem) "NewEnumerator3")))))))

(fn ConstructionScript)

(fn HandleHurt
  (params (Ratio :type Float%20%28double-precision%29)))

(fn HandleDeath
  (params (Ratio :type Float%20%28double-precision%29))
  (Collision|SetActorEnableCollision false)
  (Input|DisableInput (Variables|Default|GetPlayer%20Controller)))