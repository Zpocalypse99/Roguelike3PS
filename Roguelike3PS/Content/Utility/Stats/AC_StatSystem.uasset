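; Stat component that stores health, level and EXP values in an enum-keyed map, with functions to read, add, subtract and set them.
; Adding or subtracting current health clamps it between zero and max health, while setting writes directly without checks.
; Adding EXP triggers level-ups that carry over excess EXP, raise max health and max EXP from DT_LevelStats rows, and recheck recursively for multiple levels.
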(event `Check Min Health`
  (if (<= (`self.CheckStats` "NewEnumerator1") 0.0)
    (`self.SetStatValue` "NewEnumerator1")))

(event `Check Max Health`
  (bind _statvalue (`self.CheckStats` "NewEnumerator2"))
  (if (>= (`self.CheckStats` "NewEnumerator1") _statvalue)
    (`self.SetStatValue` "NewEnumerator1" _statvalue)))

(event `Check Max EXP`
  (bind _statvalue (`self.CheckStats` "NewEnumerator5"))
  (if (>= (`self.CheckStats` "NewEnumerator4") _statvalue)
    (`self.SubtractStatValue` "NewEnumerator4" _statvalue)
    (`self.AddStatValue` "NewEnumerator3" 1.0)
    (bind _returnvalue (`|GetDataTableRow` "/Game/Utility/Stats/DT_LevelStats.DT_LevelStats" (`KismetStringLibrary.Conv_StringToName` (`KismetStringLibrary.Concat_StrStr` "Level_" (`KismetStringLibrary.Conv_Int64ToString` (`KismetMathLibrary.Conv_DoubleToInt64` (`self.CheckStats` "NewEnumerator3"))))))
      (:`then`
        (bind (_maxhealth _maxexp) (break `/Game/Utility/Stats/FStats_List` _returnvalue))
        (`self.AddStatValue` "NewEnumerator2" _maxhealth)
        (`self.AddStatValue` "NewEnumerator5" _maxexp)
        (`self.Check Max EXP`)))))

(fn `AddStatValue`
  (params (`Select Stat` :type "/Game/Utility/Stats/Enum_Stats Enum" :default "NewEnumerator0") (AddedStatValue :type "Float (double-precision)"))
  (returns (Value :type "Float (double-precision)"))
  (bind _select_stat (`local.Select Stat`))
  (`BlueprintMapLibrary.Map_Add` (`self.Stats`) _select_stat (+ (`self.CheckStats` `Select Stat`) (`local.AddedStatValue`)))
  (switch `/Game/Utility/Stats/Enum_Stats` _select_stat
    (:`NewEnumerator0`
      _)
    (:`NewEnumerator1`
      (`self.Check Max Health`))
    (:`NewEnumerator2`
      _)
    (:`NewEnumerator3`
      _)
    (:`NewEnumerator4`
      (`self.Check Max EXP`))
    (:`NewEnumerator5`
      _))
  (return (`self.CheckStats` _select_stat)))

(fn `CheckStats`
  (params (`Select Stat` :type "/Game/Utility/Stats/Enum_Stats Enum" :default "NewEnumerator0"))
  (returns (StatValue :type "Float (double-precision)") (ReturnValue :type Boolean))
  (bind (_value _returnvalue) (`BlueprintMapLibrary.Map_Find` (`self.Stats`) `Select Stat`))
  (return _value _returnvalue))

(fn `SetStatValue`
  (params (`Select Stat` :type "/Game/Utility/Stats/Enum_Stats Enum" :default "NewEnumerator0") (`Set Value` :type "Float (double-precision)"))
  (returns (Value :type "Float (double-precision)"))
  (bind _select_stat (`local.Select Stat`))
  (`BlueprintMapLibrary.Map_Add` (`self.Stats`) `Select Stat` `Set Value`)
  (switch `/Game/Utility/Stats/Enum_Stats` _select_stat
    (:`NewEnumerator0`
      _)
    (:`NewEnumerator1`
      _)
    (:`NewEnumerator2`
      _)
    (:`NewEnumerator3`
      _)
    (:`NewEnumerator4`
      _)
    (:`NewEnumerator5`
      _))
  (return (`self.CheckStats` _select_stat)))

(fn `SubtractStatValue`
  (params (`Select Stat` :type "/Game/Utility/Stats/Enum_Stats Enum" :default "NewEnumerator0") (SubtractedValue :type "Float (double-precision)"))
  (returns (Value :type "Float (double-precision)"))
  (bind _select_stat (`local.Select Stat`))
  (`BlueprintMapLibrary.Map_Add` (`self.Stats`) _select_stat (- (`self.CheckStats` `Select Stat`) (`local.SubtractedValue`)))
  (switch `/Game/Utility/Stats/Enum_Stats` _select_stat
    (:`NewEnumerator0`
      _)
    (:`NewEnumerator1`
      (`self.Check Min Health`))
    (:`NewEnumerator2`
      _)
    (:`NewEnumerator3`
      _)
    (:`NewEnumerator4`
      _)
    (:`NewEnumerator5`
      _))
  (return (`self.CheckStats` _select_stat)))